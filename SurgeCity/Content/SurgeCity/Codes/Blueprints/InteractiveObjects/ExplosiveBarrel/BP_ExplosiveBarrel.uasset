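; Explosive barrel interactive object that damages surrounding actors when its explosion event is called.
; CE_Explosion uses a HasExploded flag to fire only once, then applies ExplosionDamage to every actor overlapping the ExplosionRad component.
; The barrel destroys itself after a short delay, provided that component is valid.
; Nothing in this graph calls the event, and the construction script is empty.
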(event Custom|CE_Explosion
  (bind _explosionrad (Variables|Default|GetExplosionRad))
  ;[1 0.3385 0.3385] Explosion Method - Custom Event
  (if (not (Variables|Default|GethasExploded))
    (Variables|Default|SethasExploded true)
    (if (Utilities|IsValid _explosionrad)
      (for _array_element (Collision|GetOverlappingActors _explosionrad 0 :!class /Script/Engine.PrimitiveComponent)
        (Game|Damage|ApplyDamage _array_element (Variables|Default|GetexplosionDamage) 0 0))
      (Utilities|FlowControl|Delay 0.2)
      (Actor|DestroyActor))))

(fn ConstructionScript)